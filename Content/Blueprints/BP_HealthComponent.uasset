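; Health component that tracks current HP against a maximum and handles incoming damage.
; ReceiveDamage subtracts the amount from HP, clamps it between zero and MaxHP, then updates HealthPercentage and the Died flag.
; Each damage call ends by firing OnHealthChanged, and the event graph holds only disabled BeginPlay and Tick stubs.
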(event EventBeginPlay)

(event EventTick
  (params (DeltaSeconds :type Float%20%28single-precision%29)))

(fn ReceiveDamage
  (params (Amount :type Float%20%28double-precision%29))
  (bind _output_get (Variables|Default|SetHP (Math|Float|Clamp(Float) (- (Variables|Default|GetHP) Amount) 0.0 (Variables|Default|GetMaxHP))))
  (Variables|Default|SetHealthPercentage (/ _output_get (Variables|Default|GetMaxHP)))
  (Variables|Default|SetDied (<= _output_get 0.0))
  (Default|CallOnHealthChanged))